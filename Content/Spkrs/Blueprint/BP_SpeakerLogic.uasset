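; Speaker product configurator logic that cycles cabinet, speaker, accent and screen finishes across a list of speakers and shows the priced result on the HUD.
; Each click handler advances a wrapping index, applies materials or a screen colour parameter, then reads that option's DataTable row by index.
; Cached descriptions and prices rebuild the HUD's choices, combined description and pound-formatted total.
; Separate functions handle music track playback, volume and stopping.
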(event EventBeginPlay)

(event Collision|EventActorBeginOverlap
  (params (OtherActor :type Actor%20Object%20Reference)))

(event EventTick
  (params (DeltaSeconds :type Float%20%28single-precision%29)))

(fn ConstructionScript)

(fn CabinetteClicked
  (bind _output_get (Variables|Default|SetCabinetteIndex (Math|Integer|%(Integer) (+ (Variables|Default|GetCabinetteIndex) 1) (Variables|Default|GetCabinetteIndexMax))))
  (switch int _output_get
    (:0
      (CallFunction|SetCabinetteMaterial "/Game/Spkrs/m/BlkGld_Cab.BlkGld_Cab"))
    (:1
      (CallFunction|SetCabinetteMaterial "/Game/Spkrs/m/WalSlv_Cab.WalSlv_Cab"))
    (:2
      (CallFunction|SetCabinetteMaterial "/Game/Spkrs/m/TkBlk_Cab.TkBlk_Cab"))
    (:3
      (CallFunction|SetCabinetteMaterial "/Game/Spkrs/m/EbStl_Cab.EbStl_Cab"))
    (:4
      (CallFunction|SetCabinetteMaterial "/Game/Spkrs/m/WhtCp_Cab.WhtCp_Cab")))
  (CallFunction|DisplayCabinetData (Variables|Default|GetCabinetteIndex)))

(fn SetCabinetteMaterial
  (params (Material :type Material%20Object%20Reference))
  (for _array_element (Variables|Default|GetSpeakerList)
    (bind _cabinetmesh (Default|GetCabinetteComponent _array_element))
    (Rendering|Material|SetMaterial _cabinetmesh 0 Material)))

(fn InitaliseSpeakerLogic
  (params (SpeakerList :type Array%20of%20BP%20Speaker%20Object%20References) (HUD :type WBP%20HUD%20Object%20Reference))
  (Utilities|FlowControl|Sequence
    (:then_0
      (Variables|Default|SetSpeakerList SpeakerList) ; Store speaker list for use in logic
    )
    (:then_1
      (Variables|Default|SetHUD HUD) ; Store Hud reference for use in logic
    )
    (:then_2
      ;[1 1 1] Initalise hud with starting data
      (CallFunction|DisplayScreenData)
      (CallFunction|DisplayAccentData)
      (CallFunction|DisplayCabinetData)
      (CallFunction|DisplaySpeakerData))))

(fn SpeakerClicked
  (bind _output_get (Variables|Default|SetSpeakerIndex (Math|Integer|%(Integer) (+ (Variables|Default|GetSpeakerIndex) 1) (Variables|Default|GetSpeakerIndexMax))))
  (switch int _output_get
    (:0
      (CallFunction|SetSpeakerMaterials "/Game/Spkrs/m/BlkGld_Twt.BlkGld_Twt" "/Game/Spkrs/m/BlkGld_Wof.BlkGld_Wof"))
    (:1
      (CallFunction|SetSpeakerMaterials "/Game/Spkrs/m/WalSlv_Twt.WalSlv_Twt" "/Game/Spkrs/m/WalSlv_Wof.WalSlv_Wof"))
    (:2
      (CallFunction|SetSpeakerMaterials "/Game/Spkrs/m/TkBlk_Twt.TkBlk_Twt" "/Game/Spkrs/m/TkBlk_Wof.TkBlk_Wof"))
    (:3
      (CallFunction|SetSpeakerMaterials "/Game/Spkrs/m/WhtCp_Twt.WhtCp_Twt" "/Game/Spkrs/m/WhtCp_Wof.WhtCp_Wof")))
  (CallFunction|DisplaySpeakerData (Variables|Default|GetSpeakerIndex)))

(fn SetSpeakerMaterials
  (params (TweeterMaterial :type Material%20Object%20Reference) (WooferMaterial :type Material%20Object%20Reference))
  (for _array_element (Variables|Default|GetSpeakerList)
    (bind (_tweetermesh _woofermesh) (Default|GetSpeakerComponents _array_element))
    (Rendering|Material|SetMaterial _tweetermesh 0 TweeterMaterial)
    (Rendering|Material|SetMaterial _woofermesh 0 WooferMaterial)))

(fn AccentClicked
  (bind _output_get (Variables|Default|SetAccentIndex (Math|Integer|%(Integer) (+ (Variables|Default|GetAccentIndex) 1) (Variables|Default|GetAccentIndexMax))))
  (switch int _output_get
    (:0
      (CallFunction|SetAccentMaterials "/Game/Spkrs/m/BlkGld_Ft.BlkGld_Ft" "/Game/Spkrs/m/BlkGld_Cab.BlkGld_Cab"))
    (:1
      (CallFunction|SetAccentMaterials "/Game/Spkrs/m/WalSlv_Ft.WalSlv_Ft" "/Game/Spkrs/m/WalSlv_Cab.WalSlv_Cab"))
    (:2
      (CallFunction|SetAccentMaterials "/Game/Spkrs/m/TkBlk_Ft.TkBlk_Ft" "/Game/Spkrs/m/TkBlk_Cab.TkBlk_Cab"))
    (:3
      (CallFunction|SetAccentMaterials "/Game/Spkrs/m/EbStl_Ft.EbStl_Ft" "/Game/Spkrs/m/EbStl_Cab.EbStl_Cab"))
    (:4
      (CallFunction|SetAccentMaterials "/Game/Spkrs/m/WhtCp_Ft.WhtCp_Ft" "/Game/Spkrs/m/WhtCp_Cab.WhtCp_Cab")))
  (CallFunction|DisplayAccentData (Variables|Default|GetAccentIndex)))

(fn SetAccentMaterials
  (params (FootMaterial :type Material%20Object%20Reference) (AccentMaterial :type Material%20Object%20Reference))
  (for _array_element (Variables|Default|GetSpeakerList)
    (bind (_footmeshes _accentmeshes) (Default|GetAccentComponents _array_element))
    (Utilities|FlowControl|Sequence
      (:then_0
        (for _array_element_2 _footmeshes
          (Rendering|Material|SetMaterial _array_element_2 0 FootMaterial)))
      (:then_1
        (for _array_element_3 _accentmeshes
          (Rendering|Material|SetMaterial _array_element_3 0 AccentMaterial))))))

(fn ScreenClicked
  (bind _output_get (Variables|Default|SetScreenIndex (Math|Integer|%(Integer) (+ (Variables|Default|GetScreenIndex) 1) (Variables|Default|GetScreenIndexMax))))
  (switch int _output_get
    (:0
      (CallFunction|SetScreenColour "0, 0, 0") ; Black
    )
    (:1
      (CallFunction|SetScreenColour "0.144100,0.115500,0.032300") ; Gold
    )
    (:2
      (CallFunction|SetScreenColour "0.089000,0.089000,0.089000") ; Dark Grey
    )
    (:3
      (CallFunction|SetScreenColour "1.000000,1.000000,1.000000") ; White
    )
    (:4
      (CallFunction|SetScreenColour "0.064200,0.023700,0.009300") ; Dark Brown
    ))
  (CallFunction|DisplayScreenData (Variables|Default|GetScreenIndex)))

(fn SetScreenColour
  (params (Colour :type Vector))
  (for _array_element (Variables|Default|GetSpeakerList)
    (bind _screenmesh (Default|GetScreenComponent _array_element))
    (Rendering|Material|SetVectorParameterValueonMaterials _screenmesh "Color" Colour)))

(fn DisplayCabinetData
  (params (Index :type Integer))
  (bind _returnvalue (Utilities|GetDataTableRow "/Game/Data/Cabinette_Data.Cabinette_Data" (Utilities|String|StringToName (Utilities|String|ToString(Integer) Index)))
    (:then
      (Utilities|FlowControl|Sequence
        (:then_0
          (Variables|Default|SetCabinetShortDescription (.ShortDescription (Utilities|Struct|BreakDT_SpeakerDataStruct _returnvalue))))
        (:then_1
          (Variables|Default|SetCabinetLongDescripition (.LongDescription (Utilities|Struct|BreakDT_SpeakerDataStruct _returnvalue))))
        (:then_2
          (Variables|Default|SetCabinetPrice (.Price (Utilities|Struct|BreakDT_SpeakerDataStruct _returnvalue))))
        (:then_3
          (CallFunction|DisplayFinalDatatoHUD))))))

(fn DisplayFinalDatatoHUD
  (Utilities|FlowControl|Sequence
    (:then_0
      ;[1 1 1] Total Price
      (Variables|/Game/HUD/WBP_HUD.WBP_HUD_C|SetTotalPrice (Variables|Default|GetHUD) (CallFunction|PriceFormatter (+ (Variables|Default|GetBasePrice) (Variables|Default|GetCabinetPrice) (Variables|Default|GetSpeakerPrice) (Variables|Default|GetAccentPrice) (Variables|Default|GetScreenPrice)))))
    (:then_1
      ;[1 1 1] Intividual Prices
      (Variables|/Game/HUD/WBP_HUD.WBP_HUD_C|SetSpeakerPrice (Variables|Default|GetHUD) (CallFunction|PriceFormatter (Variables|Default|GetSpeakerPrice)))
      (Variables|/Game/HUD/WBP_HUD.WBP_HUD_C|SetCabinetPrice (Variables|Default|GetHUD) (CallFunction|PriceFormatter (Variables|Default|GetCabinetPrice)))
      (Variables|/Game/HUD/WBP_HUD.WBP_HUD_C|SetAccentPrice (Variables|Default|GetHUD) (CallFunction|PriceFormatter (Variables|Default|GetAccentPrice)))
      (Variables|/Game/HUD/WBP_HUD.WBP_HUD_C|SetScreenPrice (Variables|Default|GetHUD) (CallFunction|PriceFormatter (Variables|Default|GetScreenPrice)))
      (Variables|/Game/HUD/WBP_HUD.WBP_HUD_C|SetBasePrice (Variables|Default|GetHUD) (CallFunction|PriceFormatter (Variables|Default|GetBasePrice))))
    (:then_2
      ;[1 1 1] Short Description
      (Variables|/Game/HUD/WBP_HUD.WBP_HUD_C|SetSpeakerChoice (Variables|Default|GetHUD) (Variables|Default|GetSpeakerShortDescription))
      (Variables|/Game/HUD/WBP_HUD.WBP_HUD_C|SetScreenChoice (Variables|Default|GetHUD) (Variables|Default|GetScreenShortDescription))
      (Variables|/Game/HUD/WBP_HUD.WBP_HUD_C|SetAccentChoice (Variables|Default|GetHUD) (Variables|Default|GetAccentShortDescription))
      (Variables|/Game/HUD/WBP_HUD.WBP_HUD_C|SetCabinetChoice (Variables|Default|GetHUD) (Variables|Default|GetCabinetShortDescription)))
    (:then_3
      ;[1 1 1] Set long discription
      (Variables|/Game/HUD/WBP_HUD.WBP_HUD_C|SetLongDescription (Variables|Default|GetHUD) (Utilities|Text|ToText(String) (Utilities|String|Append (Utilities|String|Append (Utilities|String|Append (Utilities|String|Append (Utilities|String|ToString(Text) (Variables|Default|GetSpeakerLongDescription)) " Mounted In ") (Utilities|String|ToString(Text) (Variables|Default|GetCabinetLongDescripition))) " Cabenets and ") (Utilities|String|ToString(Text) (Variables|Default|GetAccentLongDescription))))))))

(fn DisplaySpeakerData
  (params (Index :type Integer))
  (bind _returnvalue (Utilities|GetDataTableRow "/Game/Data/Speaker_Data.Speaker_Data" (Utilities|String|StringToName (Utilities|String|ToString(Integer) Index)))
    (:then
      (Utilities|FlowControl|Sequence
        (:then_0
          (Variables|Default|SetSpeakerShortDescription (.ShortDescription (Utilities|Struct|BreakDT_SpeakerDataStruct _returnvalue))))
        (:then_1
          (Variables|Default|SetSpeakerLongDescription (.LongDescription (Utilities|Struct|BreakDT_SpeakerDataStruct _returnvalue))))
        (:then_2
          (Variables|Default|SetSpeakerPrice (.Price (Utilities|Struct|BreakDT_SpeakerDataStruct _returnvalue))))
        (:then_3
          (CallFunction|DisplayFinalDatatoHUD))))))

(fn DisplayAccentData
  (params (Index :type Integer))
  (bind _returnvalue (Utilities|GetDataTableRow "/Game/Data/Accent_Data.Accent_Data" (Utilities|String|StringToName (Utilities|String|ToString(Integer) Index)))
    (:then
      (Utilities|FlowControl|Sequence
        (:then_0
          (Variables|Default|SetAccentShortDescription (.ShortDescription (Utilities|Struct|BreakDT_SpeakerDataStruct _returnvalue))))
        (:then_1
          (Variables|Default|SetAccentLongDescription (.LongDescription (Utilities|Struct|BreakDT_SpeakerDataStruct _returnvalue))))
        (:then_2
          (Variables|Default|SetAccentPrice (.Price (Utilities|Struct|BreakDT_SpeakerDataStruct _returnvalue))))
        (:then_3
          (CallFunction|DisplayFinalDatatoHUD))))))

(fn DisplayScreenData
  (params (Index :type Integer))
  (bind _returnvalue (Utilities|GetDataTableRow "/Game/Data/Screen_Data.Screen_Data" (Utilities|String|StringToName (Utilities|String|ToString(Integer) Index)))
    (:then
      (Utilities|FlowControl|Sequence
        (:then_0
          (Variables|Default|SetScreenShortDescription (.ShortDescription (Utilities|Struct|BreakDT_SpeakerDataStruct _returnvalue))))
        (:then_1
          (Variables|Default|SetScreenLongDescription (.LongDescription (Utilities|Struct|BreakDT_SpeakerDataStruct _returnvalue))))
        (:then_2
          (Variables|Default|SetScreenPrice (.Price (Utilities|Struct|BreakDT_SpeakerDataStruct _returnvalue))))
        (:then_3
          (CallFunction|DisplayFinalDatatoHUD))))))

(fn PriceFormatter
  (params (PriceInPennies :type Integer))
  (return (Class|KismetTextLibrary|AsCurrencyBase PriceInPennies "£")))

(fn PlayAudio
  (params (TrackNum :type Integer))
  (Utilities|FlowControl|Sequence
    (:then_0
      ;[1 1 1] Stop Track
      (CallFunction|StopAudio))
    (:then_1
      ;[1 1 1] Load Selected Track
      (Audio|Components|Audio|SetSound (Variables|Default|GetMusicPlayerComponent) (Utilities|Array|Get(acopy) (Variables|Default|GetTrackList) TrackNum)))
    (:then_2
      ;[1 1 1] Play Selected Track
      (CallFunction|SetAudioLevel (Variables|Default|GetAudio%20Volume))
      (Audio|Components|Audio|Play (Variables|Default|GetMusicPlayerComponent) 0.0))))

(fn SetAudioLevel
  (params (Volume :type Float%20%28single-precision%29))
  (bind _output_get (Variables|Default|SetAudio%20Volume Volume))
  (Audio|Components|Audio|AdjustVolume (Variables|Default|GetMusicPlayerComponent) 0.0 _output_get "Linear" :!class /Script/Engine.AudioComponent))

(fn StopAudio
  (Audio|Components|Audio|Stop (Variables|Default|GetMusicPlayerComponent)))