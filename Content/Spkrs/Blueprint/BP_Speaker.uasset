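; BP_Speaker is a clickable speaker actor whose mesh parts are grouped into speakers, screen, accents and cabinet.
; Clicks on each part forward to the matching event on a SpeakerLogic reference, with feet, accent plate and frame all counting as accent.
; InitialiseSpeakerBP stores that reference and shows the screen and frame cover, or hides it and ignores its collision, based on CoverActive.
; Getter functions expose the component groups.
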(event OnClicked(AccentPlate)
  (params (TouchedComponent :type Primitive%20Component%20Object%20Reference) (ButtonPressed :type Key%20Structure :default "None"))
  ;[1 1 1] Accent clicked
  (Default|AccentClicked (Variables|Default|GetSpeakerLogicRef)))

(event OnClicked(Cabinette)
  (params (TouchedComponent :type Primitive%20Component%20Object%20Reference) (ButtonPressed :type Key%20Structure :default "None"))
  ;[1 1 1] Cabinette clicked
  (Default|CabinetteClicked (Variables|Default|GetSpeakerLogicRef)))

(event OnClicked(Foot_BL)
  (params (TouchedComponent :type Primitive%20Component%20Object%20Reference) (ButtonPressed :type Key%20Structure :default "None"))
  ;[1 1 1] Accent clicked
  (Default|AccentClicked (Variables|Default|GetSpeakerLogicRef)))

(event OnClicked(Foot_BR)
  (params (TouchedComponent :type Primitive%20Component%20Object%20Reference) (ButtonPressed :type Key%20Structure :default "None"))
  ;[1 1 1] Accent clicked
  (Default|AccentClicked (Variables|Default|GetSpeakerLogicRef)))

(event OnClicked(Foot_FL)
  (params (TouchedComponent :type Primitive%20Component%20Object%20Reference) (ButtonPressed :type Key%20Structure :default "None"))
  ;[1 1 1] Accent clicked
  (Default|AccentClicked (Variables|Default|GetSpeakerLogicRef)))

(event OnClicked(Foot_FR)
  (params (TouchedComponent :type Primitive%20Component%20Object%20Reference) (ButtonPressed :type Key%20Structure :default "None"))
  ;[1 1 1] Accent clicked
  (Default|AccentClicked (Variables|Default|GetSpeakerLogicRef)))

(event OnClicked(Frame)
  (params (TouchedComponent :type Primitive%20Component%20Object%20Reference) (ButtonPressed :type Key%20Structure :default "None"))
  ;[1 1 1] Accent clicked
  (Default|AccentClicked (Variables|Default|GetSpeakerLogicRef)))

(event OnClicked(Screen)
  (params (TouchedComponent :type Primitive%20Component%20Object%20Reference) (ButtonPressed :type Key%20Structure :default "None"))
  ;[1 1 1] Screen clicked
  (Default|ScreenClicked (Variables|Default|GetSpeakerLogicRef)))

(event OnClicked(HornTweeter)
  (params (TouchedComponent :type Primitive%20Component%20Object%20Reference) (ButtonPressed :type Key%20Structure :default "None"))
  ;[1 1 1] Speakers clicked
  (Default|SpeakerClicked (Variables|Default|GetSpeakerLogicRef)))

(event OnClicked(Woofers)
  (params (TouchedComponent :type Primitive%20Component%20Object%20Reference) (ButtonPressed :type Key%20Structure :default "None"))
  ;[1 1 1] Speakers clicked
  (Default|SpeakerClicked (Variables|Default|GetSpeakerLogicRef)))

(event EventBeginPlay)

(event Collision|EventActorBeginOverlap
  (params (OtherActor :type Actor%20Object%20Reference)))

(event EventTick
  (params (DeltaSeconds :type Float%20%28single-precision%29)))

(fn ConstructionScript)

(fn GetCabinetteComponent
  (return (Variables|Default|GetCabinette)))

(fn InitialiseSpeakerBP
  (params (SpeakerLogicBP :type BP%20Speaker%20Logic%20Object%20Reference))
  (Utilities|FlowControl|Sequence
    (:then_0
      (Variables|Default|SetSpeakerLogicRef SpeakerLogicBP))
    (:then_1
      ;[1 1 1] Check Cover Active
      (if (Variables|Default|GetCoverActive)
        ;;[0 1 0.06382] Cover is active
        (Rendering|SetVisibility (Variables|Default|GetScreen) true false)
        (Rendering|SetVisibility (Variables|Default|GetFrame) true false)
        (else
          ;;[1 0.07729 0.05729] Cover is inactive
          (Rendering|SetVisibility (Variables|Default|GetFrame) false false)
          (Rendering|SetVisibility (Variables|Default|GetScreen) false false)
          (Collision|SetCollisionResponsetoAllChannels (Variables|Default|GetFrame) "ECR_Ignore")
          (Collision|SetCollisionResponsetoAllChannels (Variables|Default|GetScreen) "ECR_Ignore"))))))

(fn GetSpeakerComponents
  (return (Variables|Default|GetHornTweeter) (Variables|Default|GetWoofers)))

(fn GetAccentComponents
  (return (Utilities|Array|MakeArray (Variables|Default|GetFoot_BL) (Variables|Default|GetFoot_BR) (Variables|Default|GetFoot_FL) (Variables|Default|GetFoot_FR)) (Utilities|Array|MakeArray (Variables|Default|GetAccentPlate) (Variables|Default|GetFrame))))

(fn GetScreenComponent
  (return (Variables|Default|GetScreen)))